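; Player character for a 2D side-scroller, with X-axis movement, jumping, a HUD, pause and save/load.
; Tick picks idle, moving, jump or death flipbooks and flips control yaw from X velocity or last input direction.
; Any damage is fatal: movement stops until the death animation nearly ends, then the player respawns at the BeginPlay location.
; Saves store only the transform, loaded by key or on BeginPlay when the GameInstance flag is set.
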(event Custom|HandleAnimation
  (bind _sprite (Variables|Default|GetSprite))
  ;[0.15 0.15 0.15 0.5] Handle Animation
  (if (Variables|Default|Getisdead)
    (Sprite|SetFlipbook (Variables|Default|GetSprite) (Variables|Default|GetPlayerDeathAnimation))
    (elif (AI|Components|NavMovement|IsFalling (Variables|Character|GetCharacterMovement))
      (Sprite|SetFlipbook _sprite "/Game/Assets/Tiles/Characters/jump.jump")
      (else
        (Sprite|SetFlipbook _sprite (select (> (Math|Vector|VectorLength (Variables|/Script/Engine.MovementComponent|GetVelocity (Variables|Character|GetCharacterMovement))) 0.0) "/Game/Assets/Tiles/Characters/moving.moving" "/Game/Assets/Tiles/Characters/idle.idle"))))))

(event Custom|HandleRotation
  ;[0.15 0.15 0.15 0.5] Handl Rotation
  (Math|Float|CompareFloat (.x (Variables|/Script/Engine.MovementComponent|GetVelocity (Variables|Character|GetCharacterMovement))) 0.0
    (:>
      (Pawn|SetControlRotation (Pawn|GetController) (Math|Rotator|MakeRotator 0.0 0.0 1.8e+02) :!label _label))
    (:==
      (if (Variables|Default|Getismovingright?)
        (goto _label)
        (else
          (Pawn|SetControlRotation (Pawn|GetController) (Math|Rotator|MakeRotator 0.0 0.0 0.0) :!label _label_2))))
    (:<
      (goto _label_2))))

(event Custom|RespawnPlayerCharacter
  ;[0.15 0.15 0.15 0.5] Respawn Player
  (Transformation|SetActorLocation (Variables|Default|GetRespawnLocation) false false)
  (Variables|Default|Setisdead false)
  (Components|Activation|SetActive (Variables|Character|GetCharacterMovement) true false))

(event EventTick
  (params (DeltaSeconds :type Float%20%28single-precision%29))
  ;[0.15 0.15 0.15 0.5] Event Tick
  (CallFunction|HandleAnimation)
  (CallFunction|HandleRotation))

(event Game|Damage|EventAnyDamage
  (params (Damage :type Float%20%28single-precision%29) (DamageType :type Damage%20Type%20Object%20Reference) (InstigatedBy :type Controller%20Object%20Reference) (DamageCauser :type Actor%20Object%20Reference))
  ;[0.15 0.15 0.15 0.5] Handle Damage
  (Variables|Default|Setisdead true)
  (Components|Activation|SetActive (Variables|Character|GetCharacterMovement) false false)
  (Utilities|FlowControl|Delay (- (Class|PaperFlipbook|GetTotalDuration (Variables|Default|GetPlayerDeathAnimation)) 0.1))
  (CallFunction|RespawnPlayerCharacter))

(event EventBeginPlay
  ;[0.15 0.15 0.15 0.5] Event Begin Play Events
  (Utilities|FlowControl|Sequence
    (:then_0
      (Variables|Default|SetRespawnLocation (Transformation|GetActorLocation))
      (bind _returnvalue (UserInterface|CreateWidget "/Game/UI/Playerhud.Playerhud_C"))
      (bind _output_get (Variables|Default|Setplayerhud _returnvalue))
      (UserInterface|Viewport|AddtoViewport _output_get 0))
    (:then_1
      ;[0.15 0.15 0.15 0.5] Baturay-Menu
      (bind _asbpc_game_instance (Utilities|Casting|CastToBPC_GameInstance (Game|GetGameInstance)))
      (if (Variables|/Game/ThirdPerson/Maps/BPC_GameInstance.BPC_GameInstance_C|GetLoadVariable _asbpc_game_instance)
        (CallFunction|LoadGame)))))

(event Input|ActionEvents|InputActionJump
  (params (Key :type Key%20Structure :default "None"))
  ;[0.15 0.15 0.15 0.5] Hadle Jumping
  (:Pressed
    (Character|Jump))
  (:Released
    (Character|StopJumping)))

(event Input|AxisEvents|InputAxisMoveright
  (params (AxisValue :type Float%20%28single-precision%29))
  ;[0.15 0.15 0.15 0.5] Handle Movement
  (if (> AxisValue 0.0)
    (Variables|Default|Setismovingright? true)
    (elif (< AxisValue 0.0)
      (Variables|Default|Setismovingright? false)))
  (Pawn|Input|AddMovementInput "1.000000,0.000000,0.000000" AxisValue false))

(event Input|KeyboardEvents|DebugKeyEscape
  (params (Key :type Key%20Structure :default "None") (ActionValue :type Input%20Action%20Value%20Structure))
  ;[0.15 0.15 0.15 0.5] Baturay-Menu
  (:Pressed
    (Class|BPIPlayerControllerPause|PauseEvent(Message) (Pawn|GetController))))

(event Input|KeyboardEvents|P
  (params (Key :type Key%20Structure :default "None"))
  ;[0.15 0.15 0.15 0.5] Baturay-Menu
  (:Pressed
    (CallFunction|SaveGame)))

(event Input|KeyboardEvents|O
  (params (Key :type Key%20Structure :default "None"))
  ;[0.15 0.15 0.15 0.5] Baturay-Menu
  (:Pressed
    (CallFunction|LoadGame)))

(fn ConstructionScript)

(fn SAveGAme
  (Utilities|FlowControl|Sequence
    (:then_0
      (Utilities|IsValid (Variables|Default|GetOurSaveGameRef)
        (:Is%20Not%20Valid
          (bind _returnvalue (SaveGame|CreateSaveGameObject "/Game/ThirdPerson/Blueprints/BP_OurSaveGame.BP_OurSaveGame_C"))
          (Variables|Default|SetOurSaveGameRef _returnvalue))))
    (:then_1
      (Variables|/Game/ThirdPerson/Blueprints/BP_OurSaveGame.BP_OurSaveGame_C|SetPlayerTransform (Variables|Default|GetOurSaveGameRef) (Transformation|GetActorTransform)))
    (:then_2
      (SaveGame|SaveGametoSlot (Variables|Default|GetOurSaveGameRef) (Variables|Default|GetSaveGameSlot)))))

(fn LOadGAme
  (bind _returnvalue (Game|GetPlayerController 0))
  (bind _returnvalue_2 (SaveGame|DoesSaveGameExist (Variables|Default|GetSaveGameSlot)))
  (if _returnvalue_2
    (bind _returnvalue_3 (SaveGame|LoadGamefromSlot (Variables|Default|GetSaveGameSlot)))
    (bind _asbp_our_save_game (Utilities|Casting|CastToBP_OurSaveGame _returnvalue_3))
    (Transformation|SetActorTransform (Variables|/Game/ThirdPerson/Blueprints/BP_OurSaveGame.BP_OurSaveGame_C|GetPlayerTransform _asbp_our_save_game))
    (Input|SetInputModeGameOnly _returnvalue false)
    (Variables|/Script/Engine.PlayerController|SetbShowMouseCursor _returnvalue false)
    (else
      (Game|OpenLevel(byName) "onescreen"))))