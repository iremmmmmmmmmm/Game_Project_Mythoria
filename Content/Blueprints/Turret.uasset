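; Turret actor that fires projectiles automatically on a repeating timer.
; After an initial delay on BeginPlay, the Fire event spawns a Projectile at the Scene component's world transform with the turret as owner.
; Fire then waits the same Duration and calls itself, looping indefinitely without targeting or overlap logic.
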(event Custom|Fire
  (Game|SpawnActorfromClass "/Game/Blueprints/Projectile.Projectile_C" (Transformation|GetWorldTransform (Variables|Default|GetScene)) "Undefined" "MultiplyWithRoot" self 0)
  (Utilities|FlowControl|Delay (Variables|Default|GetDuration))
  (CallFunction|Fire))

(event EventBeginPlay
  (|CallParentFunction)
  (Utilities|FlowControl|Delay (Variables|Default|GetDuration))
  (CallFunction|Fire))

(event Collision|EventActorBeginOverlap
  (params (OtherActor :type Actor%20Object%20Reference))
  (|CallParentFunction OtherActor) ; This node is disabled and will not be called.\nDrag off pins to build functionality.
)

(event EventTick
  (params (DeltaSeconds :type Float%20%28single-precision%29))
  (|CallParentFunction DeltaSeconds) ; This node is disabled and will not be called.\nDrag off pins to build functionality.
)

(fn ConstructionScript
  (|CallParentFunction))