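; Master spike hazard, a Paper2D actor that alternates between down and up sprites and damages actors that touch it.
; BeginPlay runs an endless delay loop, timed by Duration plus a fixed pause, calling two custom events that swap the sprite.
; Box overlap always applies damage, whichever sprite shows.
; Intermediate animation frames and collision toggling exist only in disconnected nodes that never run.
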(event OnComponentBeginOverlap(Box)
  (params (OverlappedComponent :type Primitive%20Component%20Object%20Reference) (OtherActor :type Actor%20Object%20Reference) (OtherComp :type Primitive%20Component%20Object%20Reference) (OtherBodyIndex :type Integer) (bFromSweep :type Boolean) (SweepResult :type Hit%20Result%20Structure%20%28by%20ref%29))
  (Game|Damage|ApplyDamage OtherActor 1.0 0 0))

(event Custom|biringspikedown
  (Rendering|Components|Sprite|SetSprite (Variables|Default|GetPaperSprite) "/Game/Assets/spike/spike_1_Sprite.spike_1_Sprite"))

(event Custom|Bringspikeup
  (Rendering|Components|Sprite|SetSprite (Variables|Default|GetPaperSprite) "/Game/Assets/spike/spike_4_Sprite.spike_4_Sprite"))

(event EventBeginPlay
  (|CallParentFunction)
  (CallFunction|Biringspikedown :!label _label)
  (Utilities|FlowControl|Delay 0.4)
  (Utilities|FlowControl|Delay (Variables|Default|GetDuration))
  (CallFunction|Bringspikeup)
  (Utilities|FlowControl|Delay 0.4)
  (Utilities|FlowControl|Delay (Variables|Default|GetDuration))
  (goto _label))

(event Collision|EventActorBeginOverlap
  (params (OtherActor :type Actor%20Object%20Reference))
  (|CallParentFunction OtherActor) ; This node is disabled and will not be called.\nDrag off pins to build functionality.
)

(event EventTick
  (params (DeltaSeconds :type Float%20%28single-precision%29))
  (|CallParentFunction DeltaSeconds) ; This node is disabled and will not be called.\nDrag off pins to build functionality.
)

(fn ConstructionScript
  (|CallParentFunction))